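; BP_Enemy is an enemy character that tracks health and reacts to hits from the player.
; While alive, Tick clears ABP_Enemy's TakenHit flag, then polls the player's HitEnemy flag to call TakeHit.
; TakeHit feeds hit flag, alpha and direction to the anim instance and subtracts fixed health, ignoring its Damage and Location inputs.
; EndIntro sets IntroEnded; the blackboard update for it is disconnected.
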(event `EndIntro`
  (set `self.IntroEnded` true))

(event `self.ReceiveBeginPlay`)

(event `self.ReceiveTick`
  (params (DeltaSeconds :type "Float (single-precision)"))
  (if (> (`self.Health`) 0.0)
    (`|ExecutionSequence`
      (:`then_0`
        (bind _asabp_enemy (cast `/Game/Enemy/ABP_Enemy` (`SkeletalMeshComponent.GetAnimInstance` (`self.Mesh`))))
        (if (`/Game/Enemy/ABP_Enemy.TakenHit` _asabp_enemy)
          (set `/Game/Enemy/ABP_Enemy.TakenHit` false _asabp_enemy)))
      (:`then_1`
        (bind _asbp_player_character (cast `/Game/Player/BP_PlayerCharacter` (`GameplayStatics.GetPlayerCharacter` 0)))
        (if (`PlayerCharacter.HitEnemy` _asbp_player_character)
          (`self.TakeHit` 0.0 (`self.K2_GetActorLocation` _asbp_player_character))
          (set `PlayerCharacter.HitEnemy` false _asbp_player_character))))))

(fn `TakeHit`
  (params (Damage :type "Float (double-precision)") (Location :type "Vector Structure"))
  (`KismetSystemLibrary.PrintString` "Enemy Hit")
  (bind _asabp_enemy (cast `/Game/Enemy/ABP_Enemy` (`SkeletalMeshComponent.GetAnimInstance` (`self.Mesh`))))
  (set `/Game/Enemy/ABP_Enemy.TakenHit` true _asabp_enemy)
  (set `/Game/Enemy/ABP_Enemy.HitAlpha` 1.0 _asabp_enemy)
  (set `/Game/Enemy/ABP_Enemy.HitDirection` (`KismetMathLibrary.GreaterGreater_VectorRotator` (`KismetMathLibrary.GreaterGreater_VectorRotator` (- (`self.K2_GetActorLocation`) (`self.K2_GetActorLocation` (`GameplayStatics.GetPlayerCharacter` 0))) (`self.K2_GetActorRotation`)) (struct)) _asabp_enemy)
  (set `self.Health` (- (`self.Health`) 10.0)))

(fn `UserConstructionScript`)